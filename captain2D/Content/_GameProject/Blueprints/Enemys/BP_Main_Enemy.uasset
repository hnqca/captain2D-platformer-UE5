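; Base 2D side-scroller enemy character that patrols on foot, attacks the player on contact and drops loot.
; Tick drives the patrol, flipping direction and sprite when the ledge check fails or it hits a non-player obstacle.
; Damage reduces life, plays a hit animation and launches knockback based on player facing, setting a death flag at zero.
; DeathEnemy disables collision, fades the sprite via timeline, spawns mapped drops and destroys the actor.
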(event `Parent:BeginPlayer`
  (`|ExecutionSequence` :!label _label
    (:`then_0`
      (bind _returnvalue (`GameplayStatics.GetActorOfClass` "/Game/_GameProject/Blueprints/paperZD/Player/BP_Player.BP_Player_C"))
      (set `self.As BP_Player` _returnvalue))
    (:`then_2`
      (`KismetSystemLibrary.PrintString` "Hello"))))

(event `self.ReceiveBeginPlay`
  (goto _label))

(event `self.ReceiveAnyDamage`
  (params (Damage :type "Float (single-precision)") (DamageType :type "DamageType Object Reference") (InstigatedBy :type "Controller Object Reference") (DamageCauser :type "Actor Object Reference"))
  ;[1 1 1] Receive Damage
  (if (not (`self.isDeath?`))
    (bind _output_get (set `self.amountLife` (- (`self.amountLife`) Damage)))
    (`|ExecutionSequence`
      (:`then_0`
        (if (<= _output_get 0.0)
          (set `self.isDeath?` true)))
      (:`then_1`
        (`PaperZDAnimInstance.JumpToNode` (`PaperZDAnimationComponent.AnimInstance` (`self.AnimationComponent`)) "ReceiveDamage" "None"))
      (:`then_2`
        (`self.LaunchCharacter` (`KismetMathLibrary.MakeVector` (select `bool` (`/Game/_GameProject/Blueprints/paperZD/Player/BP_Player.isMovingRight?` (`self.As BP_Player`)) :`false` -150.0 :`true` 150.0) 0.0 (`KismetMathLibrary.RandomFloatInRange` 5.0 60.0)) true true)))))

(event `self.ReceiveTick`
  (params (DeltaSeconds :type "Float (single-precision)"))
  (if (and (`self.canPatrolWalking?`) (not (`self.isDeath?`))) :!label _label_2
    (`|ExecutionSequence`
      (:`then_0`
        ;[0.8275 0 1] Direção do movemento atual
        (`self.AddMovementInput` (-1.0 0.0 0.0) (select `bool` (`self.isMovingRight?`) :`false` 1.0 :`true` -1.0 :!type "Float (single-precision)")))
      (:`then_1`
        (bind _returnvalue (`self.checkLedgeWalking`))
        (if (not _returnvalue)
          (bind _isa (`/Engine/EditorBlueprintResources/StandardMacros.FlipFlop` :!label _label_3)
            (:`A`
              _)
            (:`B`
              _))
          (set `self.isMovingRight?` _isa)
          (`self.Update Direction Sprite Enemy`))))))

(event `applyPatrolWalkingMovement`
  (goto _label_2))

(event `changeMovementPatrolWalking`
  (goto _label_3))

(event `self.ReceiveHit`
  (params (MyComp :type "PrimitiveComponent Object Reference") (Other :type "Actor Object Reference") (OtherComp :type "PrimitiveComponent Object Reference") (bSelfMoved :type Boolean) (HitLocation :type "Vector Structure") (HitNormal :type "Vector Structure") (NormalImpulse :type "Vector Structure") (Hit :type "HitResult Structure (by ref)"))
  (if (== Other (`self.As BP_Player`))
    (`self.playerAttack`)
    (elif (and (!= HitNormal_X 0.0) (`self.canPatrolWalking?`))
      (`self.changeMovementPatrolWalking`))))

(event `DeathEnemy`
  (bind _sprite (`self.Sprite`))
  (bind (_returnvalue_r _returnvalue_g _returnvalue_b) (break `LinearColor` (`PaperFlipbookComponent.GetSpriteColor` _sprite)))
  (`/Engine/EditorBlueprintResources/StandardMacros.DoOnce` false
    (:`Completed`
      (`self.SetActorEnableCollision` false)
      (`PrimitiveComponent.SetMaterial` _sprite 0 "/Paper2D/TranslucentUnlitSpriteMaterial.TranslucentUnlitSpriteMaterial")
      (bind (_direction _translucent) (`Timeline|TM_Dissaper`)
        (:`Update`
          (`PaperFlipbookComponent.SetSpriteColor` (`self.Sprite`) (make `LinearColor` _returnvalue_r _returnvalue_g _returnvalue_b _translucent)))
        (:`Finished`
          (`self.DropLoot`))))))

(event `playerAttack`
  (if (not (`self.isAttacking?`))
    (set `self.isAttacking?` true)
    (set `self.canPatrolWalking?` false)
    (`PaperZDAnimInstance.JumpToNode` (`PaperZDAnimationComponent.AnimInstance` (`self.AnimationComponent`)) "PlayerAttack" "None")))

(fn `checkLedgeWalking`
  (returns (ReturnValue :type Boolean))
  (return (and (> (`KismetArrayLibrary.Array_Length` (`PrimitiveComponent.GetOverlappingActors` (`self.collisionCheckLedgeVolume`) null)) 0) (`.bWalkableFloor` (break `FindFloorResult` (`CharacterMovementComponent.CurrentFloor` (`self.CharacterMovement`)))))))

(fn `DropLoot`
  (bind _itemstodrop (`self.itemsToDrop`))
  (if (> (`BlueprintMapLibrary.Map_Length` (`self.itemsToDrop`)) 0)
    (bind _keys (`BlueprintMapLibrary.Map_Keys` _itemstodrop))
    (for _array_element _keys
      (for _ (range 1 (+ (`BlueprintMapLibrary.Map_Find` _itemstodrop _array_element) 1))
        (`|SpawnActorFromClass` _array_element (`self.GetTransform`) "Undefined" "MultiplyWithRoot" null null))))
  (`self.K2_DestroyActor`))

(fn `Update Direction Sprite Enemy`
  (`SceneComponent.K2_SetWorldRotation` (`self.Sprite`) (`KismetMathLibrary.MakeRotator` 0.0 0.0 (select `bool` (`self.isMovingRight?`) :`true` 180.0)) false false))

(fn `UserConstructionScript`)