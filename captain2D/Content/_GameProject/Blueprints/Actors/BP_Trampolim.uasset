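; BP_Trampolim is a trampoline actor that launches the player upward when they touch it.
; On overlap with BP_Player, a DoOnce plays the flipbook from the start while a Delay loop polls for a specific frame to fire LaunchCharacter with Z override.
; A parallel delay freezes the flipbook after its length elapses.
; The player leaving the collision resets the DoOnce.
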(event `self.collisionDetectPlayer.OnComponentBeginOverlap`
  (params (OverlappedComponent :type "PrimitiveComponent Object Reference") (OtherActor :type "Actor Object Reference") (OtherComp :type "PrimitiveComponent Object Reference") (OtherBodyIndex :type Integer) (bFromSweep :type Boolean) (SweepResult :type "HitResult Structure (by ref)"))
  (bind _rendercomponent (`self.RenderComponent`))
  (bind _asbp_player (cast `/Game/_GameProject/Blueprints/paperZD/Player/BP_Player` OtherActor))
  (`/Engine/EditorBlueprintResources/StandardMacros.DoOnce` false :!label _label
    (:`Completed`
      (`|ExecutionSequence`
        (:`then_0`
          (`PaperFlipbookComponent.PlayFromStart` _rendercomponent))
        (:`then_1`
          (`PaperFlipbookComponent.SetPlayRate` _rendercomponent 1.0)
          (`|ExecutionSequence`
            (:`then_0`
              (if (== (`PaperFlipbookComponent.GetPlaybackPositionInFrames` _rendercomponent) 3) :!label _label_2
                (`Character.LaunchCharacter` _asbp_player (0.0 0.0 500.0) false true)
                (else
                  (`KismetSystemLibrary.Delay` 0.1)
                  (goto _label_2))))
            (:`then_1`
              (`KismetSystemLibrary.Delay` (`PaperFlipbookComponent.GetFlipbookLength` _rendercomponent))
              (`PaperFlipbookComponent.SetPlayRate` _rendercomponent 0.0))))))))

(event `self.collisionDetectPlayer.OnComponentEndOverlap`
  (params (OverlappedComponent :type "PrimitiveComponent Object Reference") (OtherActor :type "Actor Object Reference") (OtherComp :type "PrimitiveComponent Object Reference") (OtherBodyIndex :type Integer))
  (cast `/Game/_GameProject/Blueprints/paperZD/Player/BP_Player` OtherActor)
  (goto _label :!via `Reset`))

(fn `UserConstructionScript`)