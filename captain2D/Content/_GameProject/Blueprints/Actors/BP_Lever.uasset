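; BP_Lever is a one-shot lever that the player switches on with E while overlapping its collision, which enables and disables the lever's input.
; On first use it swaps its Paper2D sprite to the on state and runs InteractionLever over a list of actor classes.
; For each class, it finds one world instance and, if tagged "leverInteract", calls that actor's leverInteract function by name through a short timer, otherwise printing an error.
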(event `self.collisionDetectPlayer.OnComponentBeginOverlap`
  (params (OverlappedComponent :type "PrimitiveComponent Object Reference") (OtherActor :type "Actor Object Reference") (OtherComp :type "PrimitiveComponent Object Reference") (OtherBodyIndex :type Integer) (bFromSweep :type Boolean) (SweepResult :type "HitResult Structure (by ref)"))
  (cast `/Game/_GameProject/Blueprints/paperZD/Player/BP_Player` OtherActor)
  (`self.EnableInput` (`GameplayStatics.GetPlayerController` 0)))

(event `Key|E`
  (params (Key :type "Key Structure"))
  (:`Pressed`
    (`/Engine/EditorBlueprintResources/StandardMacros.DoOnce` false
      (:`Completed`
        (if (not (`self.isActive?`))
          (set `self.isActive?` true)
          (`PaperSpriteComponent.SetSprite` (`self.PaperSprite`) "/Game/_GameProject/Assets/lever/sprite_lever_on.sprite_lever_on")
          (`self.interactionLever`))))))

(event `self.collisionDetectPlayer.OnComponentEndOverlap`
  (params (OverlappedComponent :type "PrimitiveComponent Object Reference") (OtherActor :type "Actor Object Reference") (OtherComp :type "PrimitiveComponent Object Reference") (OtherBodyIndex :type Integer))
  (cast `/Game/_GameProject/Blueprints/paperZD/Player/BP_Player` OtherActor)
  (`self.DisableInput` (`GameplayStatics.GetPlayerController` 0)))

(fn `interactionLever`
  (for _array_element (`self.actorsInteractingWithTheLever`)
    (if (`KismetSystemLibrary.IsValidClass` _array_element)
      (bind _returnvalue (`GameplayStatics.GetActorOfClass` _array_element))
      (if (`self.ActorHasTag` _returnvalue "leverInteract")
        (`KismetSystemLibrary.K2_SetTimer` _returnvalue "leverInteract" 0.1)
        (else
          (`KismetSystemLibrary.PrintString` "ERROR: The defined class does not have \"leverInteract\" tag")))
      (else
        (`KismetSystemLibrary.PrintString` "ERROR: Class reference is not valid (BP_Lever)")))))

(fn `UserConstructionScript`)