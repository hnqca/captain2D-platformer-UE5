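; Level exit door that opens once the player has collected every key in the level.
; It counts key actors on BeginPlay and shows a collected/total counter that updates on each key pickup.
; When the player overlaps it with all keys, it plays the opening flipbook once, then calls the persistent game instance to advance the level.
; That overlap also enables input on the door until the player leaves.
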(event `onKeyPickup`
  ;[1 1 1] Update the remaining keys needed to open the door when a key is collected.
  (bind _result (`/Engine/EditorBlueprintResources/StandardMacros.IncrementInt` (`self.collectedKeyCount`))
    (:`  `
      (set `self.collectedKeyCount` _result)
      (`self.updateKeyCountText`))))

(event `updateKeyCountText`
  ;[1 1 1] Update the text displaying the remaining key count
  (`TextRenderComponent.K2_SetText` (`self.TxtAmountKeys`) (`KismetTextLibrary.Conv_StringToText` (`KismetStringLibrary.BuildString_Int` (`KismetStringLibrary.Conv_IntToString` (`self.collectedKeyCount`)) "/" (`self.totalKeysInTheLevel`)))))

(event `self.ReceiveBeginPlay`
  ;[1 1 1] Keep track of how many keys are scattered throughout the level
  (bind _outactors (`GameplayStatics.GetAllActorsOfClass` "/Game/_GameProject/Blueprints/Actors/BP_Key_Door.BP_Key_Door_C"))
  (set `self.totalKeysInTheLevel` (`KismetArrayLibrary.Array_Length` _outactors))
  (`self.updateKeyCountText`))

(event `self.collisionDetectPlayer.OnComponentBeginOverlap`
  (params (OverlappedComponent :type "PrimitiveComponent Object Reference") (OtherActor :type "Actor Object Reference") (OtherComp :type "PrimitiveComponent Object Reference") (OtherBodyIndex :type Integer) (bFromSweep :type Boolean) (SweepResult :type "HitResult Structure (by ref)"))
  (bind _rendercomponent (`self.RenderComponent`))
  ;[1 1 1] Check if all the level's keys have been collected, if true, unlock the door.
  (cast `/Game/_GameProject/Blueprints/paperZD/Player/BP_Player` OtherActor)
  (if (== (`self.collectedKeyCount`) (`self.totalKeysInTheLevel`))
    (`|ExecutionSequence`
      (:`then_0`
        (`/Engine/EditorBlueprintResources/StandardMacros.DoOnce` false
          (:`Completed`
            (`PaperFlipbookComponent.SetLooping` _rendercomponent false)
            (`PaperFlipbookComponent.SetFlipbook` _rendercomponent "/Game/_GameProject/Assets/Pirate_Ship/Sprites/Decorations/Door/Opening/FB-LevelDoor_Opening.FB-LevelDoor_Opening")
            (`KismetSystemLibrary.Delay` (`PaperFlipbookComponent.GetFlipbookLength` _rendercomponent))
            (`self.teleportPlayerToNextLevel`))))
      (:`then_1`
        (`self.EnableInput` (`GameplayStatics.GetPlayerController` 0))))))

(event `self.collisionDetectPlayer.OnComponentEndOverlap`
  (params (OverlappedComponent :type "PrimitiveComponent Object Reference") (OtherActor :type "Actor Object Reference") (OtherComp :type "PrimitiveComponent Object Reference") (OtherBodyIndex :type Integer))
  (cast `/Game/_GameProject/Blueprints/paperZD/Player/BP_Player` OtherActor)
  (`self.DisableInput` (`GameplayStatics.GetPlayerController` 0)))

(event `teleportPlayerToNextLevel`
  ;[1 1 1] Teleport the player to the next level
  (`/Engine/EditorBlueprintResources/StandardMacros.DoOnce` false
    (:`Completed`
      (bind _asgame_instance_persistent_vars (cast `/Game/_GameProject/Blueprints/GameInstance_PersistentVars` (`GameplayStatics.GetGameInstance`)))
      (`/Game/_GameProject/Blueprints/GameInstance_PersistentVars.updateCurrentLevel` _asgame_instance_persistent_vars true))))

(fn `UserConstructionScript`)