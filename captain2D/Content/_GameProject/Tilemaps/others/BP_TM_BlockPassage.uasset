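; BP_TM_BlockPassage is a tilemap passage blocker that toggles between open and closed, with a lever-interact entry point.
; The TogglePassage event flips IsOpen, switching the render component's collision off when opening and to query-only when closing.
; A timeline plays forward on opening and in reverse on closing, driving the tilemap color's alpha while preserving its RGB.
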(event `togglePassage (open/close)`
  (bind (_returnvalue_r _returnvalue_g _returnvalue_b) (break `LinearColor` (`PaperTileMapComponent.GetTileMapColor` (`self.RenderComponent`))))
  (if (`self.isOpen?`)
    (set `self.isOpen?` false)
    (`PrimitiveComponent.SetCollisionEnabled` (`self.RenderComponent`) "QueryOnly")
    (bind (_direction _newtrack_0) (`Timeline|Timeline` :!via `ReverseFromEnd` :!label _label)
      (:`Update`
        (`PaperTileMapComponent.SetTileMapColor` (`self.RenderComponent`) (make `LinearColor` _returnvalue_r _returnvalue_g _returnvalue_b _newtrack_0))))
    (else
      (set `self.isOpen?` true)
      (`PrimitiveComponent.SetCollisionEnabled` (`self.RenderComponent`) "NoCollision")
      (goto _label :!via `PlayFromStart`))))

(fn `leverInteract`
  (`self.togglePassage (open/close)`))

(fn `UserConstructionScript`)